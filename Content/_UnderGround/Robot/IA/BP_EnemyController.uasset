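; AI controller for the enemy that runs BT_Enemy and feeds it what its perception knows about the player.
; On BeginPlay it starts the tree only if its owner casts to BP_Enemi.
; Sensing a FirstPersonCharacter sets the PlayerRef blackboard key; losing it stores the stimulus location as LastPlayerLocation and clears PlayerRef.
; A ResetPlayerRef event also clears that key.
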(event `self.ReceiveBeginPlay`
  (bind _asbp_enemi (cast `/Game/_UnderGround/Robot/BP_Enemi` (`self.GetOwner`)))
  (set `self.As BP Enemi` _asbp_enemi)
  (`self.RunBehaviorTree` "/Game/_UnderGround/Robot/IA/BT_Enemy.BT_Enemy"))

(event `self.AIPerception.OnTargetPerceptionUpdated`
  (params (Actor :type "Actor Object Reference") (Stimulus :type "AIStimulus Structure"))
  (bind _asfirst_person_character (cast `/Game/_UnderGround/Player/Blueprint/FirstPersonCharacter` Actor))
  (if true
    (if Stimulus_bSuccessfullySensed
      (`BlackboardComponent.SetValueAsObject` (`AIBlueprintHelperLibrary.GetBlackboard` null) (`KismetStringLibrary.Conv_StringToName` "PlayerRef") _asfirst_person_character)
      (else
        (`BlackboardComponent.SetValueAsVector` (`AIBlueprintHelperLibrary.GetBlackboard` null) (`KismetStringLibrary.Conv_StringToName` "LastPlayerLocation") Stimulus_StimulusLocation)
        (`BlackboardComponent.ClearValue` (`AIBlueprintHelperLibrary.GetBlackboard` null) (`KismetStringLibrary.Conv_StringToName` "PlayerRef"))))))

(event `ResetPlayerRef`
  (`BlackboardComponent.ClearValue` (`AIBlueprintHelperLibrary.GetBlackboard` null) (`KismetStringLibrary.Conv_StringToName` "PlayerRef")))

(fn `UserConstructionScript`)