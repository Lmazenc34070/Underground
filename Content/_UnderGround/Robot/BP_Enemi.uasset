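; BP_Enemi is an enemy robot powered by nearby light: the player's active light or a lit WallLight inside DetectELectric.
; Tick refills stamina while powered, and timelines drain it once power is lost.
; Stamina scales walk speed and drives IsOn, halting movement and rotation at zero.
; RunQTE either bugs the robot temporarily when the player's QTE count is high enough, or screams and respawns the player.
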(event `self.DetectELectric.OnComponentBeginOverlap`
  (params (OverlappedComponent :type "PrimitiveComponent Object Reference") (OtherActor :type "Actor Object Reference") (OtherComp :type "PrimitiveComponent Object Reference") (OtherBodyIndex :type Integer) (bFromSweep :type Boolean) (SweepResult :type "HitResult Structure (by ref)"))
  ;[1 1 1] Gain Stamina
  (bind _asfirst_person_character (cast `/Game/_UnderGround/Player/Blueprint/FirstPersonCharacter` OtherActor)
    (:`then`
      (bind _output_get (set `self.PlayerRef` _asfirst_person_character))
      (if (`/Game/_UnderGround/Player/Blueprint/FirstPersonCharacter.lightIsOn` _output_get)
        (`TimelineComponent.Stop` (`self.RatioStamina`))))
    (:`CastFailed`
      (bind _aswall_light (cast `/Game/_UnderGround/Mechanics/Lights/WallLight` OtherActor))
      (set `self.As Wall Light` _aswall_light))))

(event `self.DetectELectric.OnComponentEndOverlap`
  (params (OverlappedComponent :type "PrimitiveComponent Object Reference") (OtherActor :type "Actor Object Reference") (OtherComp :type "PrimitiveComponent Object Reference") (OtherBodyIndex :type Integer))
  ;[1 1 1] Perte Stamina
  (`self.RatioStamina__UpdateFunc`)
  (`|ExecutionSequence`
    (:`then_0`
      (bind _asfirst_person_character (cast `/Game/_UnderGround/Player/Blueprint/FirstPersonCharacter` OtherActor)
        (:`then`
          (set `self.PlayerRef` null)
          (if (`/Game/_UnderGround/Player/Blueprint/FirstPersonCharacter.lightIsOn` _asfirst_person_character)
            (`TimelineComponent.SetPlayRate` (`self.RatioStamina`) (/ 1.0 (`self.VitessePerteStamina`)) :!label _label)
            (bind (_direction _stamina) (`Timeline|RatioStamina` :!via `PlayFromStart`)
              (:`Update`
                (set `self.Stamina` _stamina))
              (:`Finished`
                (set `self.FirstTimePenetrated?` true)))))
        (:`CastFailed`
          (bind _aswall_light (cast `/Game/_UnderGround/Mechanics/Lights/WallLight` OtherActor))
          (set `self.As Wall Light` null)
          (if (> (`LightComponentBase.Intensity` (`/Game/_UnderGround/Mechanics/Lights/WallLight.PointLight` _aswall_light)) 0.0)
            (goto _label)))))))

(event `self.ReceiveTick`
  (params (DeltaSeconds :type "Float (single-precision)"))
  (bind _charactermovement (`self.CharacterMovement`))
  (bind _charactermovement_2 (`self.CharacterMovement`))
  ;[1 1 1] Ratio Vitesse/Stamina
  (if (<= (`self.Stamina`) 0.0)
    (set `CharacterMovementComponent.RotationRate` (struct) _charactermovement)
    (set `CharacterMovementComponent.MaxWalkSpeed` 0.0 _charactermovement_2)
    (else
      (set `CharacterMovementComponent.RotationRate` (struct :`Yaw` 360.0) _charactermovement)
      (set `CharacterMovementComponent.MaxWalkSpeed` (* (`self.SpeedWalkingMax`) (`self.Stamina`)) _charactermovement_2)))
  (if (> (`self.Stamina`) 0.0)
    (set `self.isOn` true)
    (else
      (set `self.isOn` false)))
  ;;[1 1 1] Debug
  (`KismetSystemLibrary.PrintString` (`KismetStringLibrary.Conv_DoubleToString` (`self.Stamina`)) true true (struct :`G` 0.66 :`B` 1.0 :`A` 1.0) 0.0)
  (`KismetSystemLibrary.PrintString` (`KismetStringLibrary.Conv_DoubleToString` (`CharacterMovementComponent.MaxWalkSpeed` (`self.CharacterMovement`))) true true (struct :`R` 1.0 :`G` 0.016606 :`A` 1.0) 0.0)
  (`/Engine/EditorBlueprintResources/StandardMacros.IsValid` (`self.PlayerRef`)
    (:`Is Valid`
      (`KismetSystemLibrary.PrintString` "IsValid" true true (struct :`G` 0.66 :`B` 1.0 :`A` 1.0) 0.0)
      (if (`/Game/_UnderGround/Player/Blueprint/FirstPersonCharacter.lightIsOn` (`self.PlayerRef`))
        (`self.RatioStamina__FinishedFunc`)
        (set `self.Stamina` 1.0)
        (set `self.SpeedWalkingMax` 300.0)
        (`TimelineComponent.Stop` (`self.Timeline_0`))
        (goto _label_2 :!via `Reset`)
        (elif (`self.FirstTimePenetrated?`)
          (`/Engine/EditorBlueprintResources/StandardMacros.DoOnce` false :!label _label_2
            (:`Completed`
              (`TimelineComponent.SetPlayRate` (`self.Timeline_0`) (/ 1.0 (`self.VitessePerteStamina`)))
              (bind (_direction _stamina) (`Timeline|Timeline_0` :!via `PlayFromStart`)
                (:`Update`
                  (set `self.Stamina` _stamina))
                (:`Finished`
                  (set `self.FirstTimePenetrated?` true))))))))
    (:`Is Not Valid`
      (`/Engine/EditorBlueprintResources/StandardMacros.IsValid` (`self.As Wall Light`)
        (:`Is Valid`
          (if (> (`LightComponentBase.Intensity` (`/Game/_UnderGround/Mechanics/Lights/WallLight.PointLight` (`self.As Wall Light`))) 0.0)
            (`self.RatioStamina__FinishedFunc`)
            (set `self.Stamina` 1.0)
            (set `self.SpeedWalkingMax` 300.0)
            (`TimelineComponent.Stop` (`self.Timeline_0`))
            (`TimelineComponent.Stop` (`self.RatioStamina`))
            (goto _label_2 :!via `Reset`)
            (else
              (goto _label_2))))))))

(event `/Game/_UnderGround/Mechanics/BPI_QTE.RunQTE`
  (bind _playerref (`self.PlayerRef`))
  ;[1 1 1] Ratio Vitesse/Stamina
  (if (>= (`/Game/_UnderGround/Player/Blueprint/FirstPersonCharacter.QTE_Count` _playerref) 15)
    (set `self.inBug?` true)
    (`KismetSystemLibrary.Delay` 5.0)
    (set `self.inBug?` false)
    (else
      (set `self.SCREAM` true)
      (`KismetSystemLibrary.Delay` 1.0)
      (set `self.SCREAM` false)
      (`/Game/_UnderGround/Player/Blueprint/FirstPersonCharacter.Respawn` _playerref))))

(fn `UserConstructionScript`)