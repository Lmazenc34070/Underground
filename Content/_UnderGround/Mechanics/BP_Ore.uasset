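; BP_Ore is an ore actor whose point light is tinted by OreColor in the construction script and pulses during play.
; On BeginPlay, Aura retries a random roll every 0.4 seconds with a rising bias, giving each ore a random start delay.
; A timeline then drives the light intensity, and a FlipFlop on its finish alternates reverse and forward playback to keep the glow looping.
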(event `Aura`
  (if (>= (+ (`KismetMathLibrary.RandomFloat`) (`self.ValueR`)) 0.8) :!label _label
    (bind (_direction _light) (`Timeline|Timeline_0` :!label _label_2)
      (:`Update`
        (`LightComponent.SetIntensity` (`self.PointLight`) (`KismetMathLibrary.Lerp` 50.0 100.0 _light)))
      (:`Finished`
        (`/Engine/EditorBlueprintResources/StandardMacros.FlipFlop`
          (:`A`
            (goto _label_2 :!via `ReverseFromEnd`))
          (:`B`
            (goto _label_2 :!via `PlayFromStart`)))))
    (else
      (`KismetSystemLibrary.Delay` 0.4)
      (set `self.ValueR` (+ (`self.ValueR`) 0.1))
      (goto _label))))

(event `self.ReceiveBeginPlay`
  (`self.Aura`))

(fn `UserConstructionScript`
  (`LightComponent.SetLightColor` (`self.PointLight`) (`self.OreColor`) true))