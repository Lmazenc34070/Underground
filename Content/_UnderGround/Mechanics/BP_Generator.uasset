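; Interactable generator that, when the player carries a fuse, powers up by showing fuse meshes, playing sound and locking itself as lit.
; Interact passes the fuse check, which tests Fusible1 against itself, to every BP_Gate and to WallLight flicker.
; A first attempt without the fuse only plays a different sound and updates the lights.
; Overlap zones drive the "Activate" prompt and a Tick-based, distance-mapped sphere opacity while unlit.
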(event `self.ReceiveBeginPlay`
  (`SceneComponent.SetVisibility` (`self.Fusible_Proto_v1_PS4_Combine`) false false)
  (`SceneComponent.SetVisibility` (`self.Fusible_Proto_v1_PS4_Combine1`) false false))

(event `/Game/_UnderGround/Mechanics/BPI_Interatable.Interact`
  (bind _returnvalue (`self.K2_GetActorLocation`))
  (if (not (`self.lit`))
    (bind _asfirst_person_character (cast `/Game/_UnderGround/Player/Blueprint/FirstPersonCharacter` (`GameplayStatics.GetPlayerPawn` 0)))
    (bind _outactors (`GameplayStatics.GetAllActorsOfClass` "/Game/_UnderGround/Mechanics/BP_Gate.BP_Gate_C"))
    (for _array_element _outactors
      (bind _returnvalue_2 (and (`/Game/_UnderGround/Player/Blueprint/FirstPersonCharacter.Fusible1` _asfirst_person_character) (`/Game/_UnderGround/Player/Blueprint/FirstPersonCharacter.Fusible1` _asfirst_person_character)))
      (`/Game/_UnderGround/Mechanics/BP_Gate.OpeningTrigger` _array_element _returnvalue_2)
      (set `self.inZone` false)
      (`MeshComponent.SetVectorParameterValueOnMaterials` (`self.Sphere1`) "Opacity" (0.0 0.0 0.0))
      (bind _outactors_2 (`GameplayStatics.GetAllActorsOfClass` "/Game/_UnderGround/Mechanics/Lights/WallLight.WallLight_C"))
      (for _ _outactors_2
        (if _returnvalue_2
          (`GameplayStatics.PlaySoundAtLocation` "/Game/_UnderGround/Sounds/generator_2.generator_2" _returnvalue (struct) 0.05 1.0 0.0 null null null null)
          (`SceneComponent.SetVisibility` (`self.Fusible_Proto_v1_PS4_Combine`) true false)
          (`SceneComponent.SetVisibility` (`self.Fusible_Proto_v1_PS4_Combine1`) true false)
          (`AudioComponent.Play` (`self.AudioDepose`) 0.0)
          (`MeshComponent.SetVectorParameterValueOnMaterials` (`self.Sphere1`) "Opacity" (0.0 0.0 0.0))
          (set `self.lit` true)
          (bind _asfirst_person_character_2 (cast `/Game/_UnderGround/Player/Blueprint/FirstPersonCharacter` (`GameplayStatics.GetPlayerPawn` 0)))
          (`Widget.SetVisibility` (`/Game/_UnderGround/Player/Blueprint/FirstPersonCharacter.Interact` _asfirst_person_character_2) "Hidden")
          (`/Game/_UnderGround/Mechanics/Lights/WallLight.SetFlick` _outactors_2 _returnvalue_2 :!label _label)
          (elif (not (`self.FirstTryOpening`))
            (`GameplayStatics.PlaySoundAtLocation` "/Game/_UnderGround/Sounds/generator_1.generator_1" _returnvalue (struct) 0.05 1.0 0.0 null null null null)
            (set `self.FirstTryOpening` true)
            (goto _label)))))))

(event `self.InteracterZone.OnComponentBeginOverlap`
  (params (OverlappedComponent :type "PrimitiveComponent Object Reference") (OtherActor :type "Actor Object Reference") (OtherComp :type "PrimitiveComponent Object Reference") (OtherBodyIndex :type Integer) (bFromSweep :type Boolean) (SweepResult :type "HitResult Structure (by ref)"))
  (bind _asfirst_person_character (cast `/Game/_UnderGround/Player/Blueprint/FirstPersonCharacter` OtherActor))
  (set `self.As First Person Character` _asfirst_person_character)
  (set `self.inZone` true))

(event `self.InteracterZone.OnComponentEndOverlap`
  (params (OverlappedComponent :type "PrimitiveComponent Object Reference") (OtherActor :type "Actor Object Reference") (OtherComp :type "PrimitiveComponent Object Reference") (OtherBodyIndex :type Integer))
  (set `self.inZone` false)
  (`MeshComponent.SetVectorParameterValueOnMaterials` (`self.Sphere1`) "Opacity" (0.0 0.0 0.0)))

(event `self.ReceiveTick`
  (params (DeltaSeconds :type "Float (single-precision)"))
  (bind (_returnvalue_x _returnvalue_y) (`KismetMathLibrary.BreakVector` (`SceneComponent.K2_GetComponentLocation` (`self.Sphere1`))))
  (bind (_returnvalue_x_2 _returnvalue_y_2) (`KismetMathLibrary.BreakVector` (`SceneComponent.K2_GetComponentLocation` (`Character.CapsuleComponent` (`self.As First Person Character`)))))
  (bind _returnvalue (/ (+ (`KismetMathLibrary.Abs` (- _returnvalue_x _returnvalue_x_2)) (`KismetMathLibrary.Abs` (- _returnvalue_y _returnvalue_y_2))) 2.0))
  (if (and (`self.inZone`) (not (`self.lit`)))
    (if (>= _returnvalue 250.0)
      (`MeshComponent.SetVectorParameterValueOnMaterials` (`self.Sphere1`) "Opacity" (`KismetMathLibrary.MakeVector` (`KismetMathLibrary.MapRangeClamped` _returnvalue 250.0 266.0 1.0)))
      (else
        (`MeshComponent.SetVectorParameterValueOnMaterials` (`self.Sphere1`) "Opacity" (`KismetMathLibrary.MakeVector` (`KismetMathLibrary.MapRangeClamped` _returnvalue 40.0 200.0 0.0 1.0)))))))

(event `self.Inter.OnComponentBeginOverlap`
  (params (OverlappedComponent :type "PrimitiveComponent Object Reference") (OtherActor :type "Actor Object Reference") (OtherComp :type "PrimitiveComponent Object Reference") (OtherBodyIndex :type Integer) (bFromSweep :type Boolean) (SweepResult :type "HitResult Structure (by ref)"))
  (bind _asfirst_person_character (cast `/Game/_UnderGround/Player/Blueprint/FirstPersonCharacter` OtherActor))
  (if (and (not (`self.lit`)) (`KismetStringLibrary.EqualEqual_StrStr` (`KismetSystemLibrary.GetDisplayName` (`Character.CapsuleComponent` _asfirst_person_character)) (`KismetSystemLibrary.GetDisplayName` OtherComp)))
    (`/Game/_UnderGround/InterfaceBP/Hud_Interactions/HUD_Interact.ChangeName` (`/Game/_UnderGround/Player/Blueprint/FirstPersonCharacter.Interact` _asfirst_person_character) "Activate")))

(event `self.Inter.OnComponentEndOverlap`
  (params (OverlappedComponent :type "PrimitiveComponent Object Reference") (OtherActor :type "Actor Object Reference") (OtherComp :type "PrimitiveComponent Object Reference") (OtherBodyIndex :type Integer))
  (bind _asfirst_person_character (cast `/Game/_UnderGround/Player/Blueprint/FirstPersonCharacter` OtherActor))
  (if (`KismetStringLibrary.EqualEqual_StrStr` (`KismetSystemLibrary.GetDisplayName` (`Character.CapsuleComponent` _asfirst_person_character)) (`KismetSystemLibrary.GetDisplayName` OtherComp))
    (`Widget.SetVisibility` (`/Game/_UnderGround/Player/Blueprint/FirstPersonCharacter.Interact` _asfirst_person_character) "Hidden")))

(fn `UserConstructionScript`)