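; BP_Rustine is an actor that fades a sphere's material based on how close the first-person character is.
; Sphere2 overlaps store the character and toggle InZone, with any actor leaving clearing the flag.
; While InZone, Tick averages the absolute X and Y offsets from Sphere1, ignoring height.
; That distance drives the "Opacity" parameter through two clamped ramps, peaking at mid range and fading out nearer or farther.
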(event `self.Sphere2.OnComponentEndOverlap`
  (params (OverlappedComponent :type "PrimitiveComponent Object Reference") (OtherActor :type "Actor Object Reference") (OtherComp :type "PrimitiveComponent Object Reference") (OtherBodyIndex :type Integer))
  (set `self.inZone` false))

(event `self.Sphere2.OnComponentBeginOverlap`
  (params (OverlappedComponent :type "PrimitiveComponent Object Reference") (OtherActor :type "Actor Object Reference") (OtherComp :type "PrimitiveComponent Object Reference") (OtherBodyIndex :type Integer) (bFromSweep :type Boolean) (SweepResult :type "HitResult Structure (by ref)"))
  (bind _asfirst_person_character (cast `/Game/_UnderGround/Player/Blueprint/FirstPersonCharacter` OtherActor))
  (set `self.As First Person Character` _asfirst_person_character)
  (set `self.inZone` true))

(event `self.ReceiveTick`
  (params (DeltaSeconds :type "Float (single-precision)"))
  (bind (_returnvalue_x _returnvalue_y) (`KismetMathLibrary.BreakVector` (`SceneComponent.K2_GetComponentLocation` (`self.Sphere1`))))
  (bind (_returnvalue_x_2 _returnvalue_y_2) (`KismetMathLibrary.BreakVector` (`SceneComponent.K2_GetComponentLocation` (`Character.CapsuleComponent` (`self.As First Person Character`)))))
  (bind _returnvalue (/ (+ (`KismetMathLibrary.Abs` (- _returnvalue_x _returnvalue_x_2)) (`KismetMathLibrary.Abs` (- _returnvalue_y _returnvalue_y_2))) 2.0))
  (if (`self.inZone`)
    (if (>= _returnvalue 210.0)
      (`MeshComponent.SetVectorParameterValueOnMaterials` (`self.Sphere1`) "Opacity" (`KismetMathLibrary.MakeVector` (`KismetMathLibrary.MapRangeClamped` _returnvalue 210.0 250.0 1.0)))
      (else
        (`MeshComponent.SetVectorParameterValueOnMaterials` (`self.Sphere1`) "Opacity" (`KismetMathLibrary.MakeVector` (`KismetMathLibrary.MapRangeClamped` _returnvalue 100.0 150.0 0.0 1.0)))))))

(fn `UserConstructionScript`
  (`parent.UserConstructionScript`))