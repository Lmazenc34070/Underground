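; Collapse trigger that plays a level sequence when the first-person character's capsule enters its box while Fall is false.
; On trigger it turns on the character's QTE flag, hides the torch and starts the sequence.
; It also makes Box1 block all channels and shifts the player capsule back along world X.
; After a fixed delay it clears QTE and shows the torch again; Fall is never set in this graph.
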(event `self.BoxTrigger.OnComponentBeginOverlap`
  (params (OverlappedComponent :type "PrimitiveComponent Object Reference") (OtherActor :type "Actor Object Reference") (OtherComp :type "PrimitiveComponent Object Reference") (OtherBodyIndex :type Integer) (bFromSweep :type Boolean) (SweepResult :type "HitResult Structure (by ref)"))
  (if (not (`self.Fall`))
    (bind _asfirst_person_character (cast `/Game/_UnderGround/Player/Blueprint/FirstPersonCharacter` OtherActor))
    (if (`KismetStringLibrary.EqualEqual_StrStr` (`KismetSystemLibrary.GetDisplayName` (`Character.CapsuleComponent` _asfirst_person_character)) (`KismetSystemLibrary.GetDisplayName` OtherComp))
      (set `/Game/_UnderGround/Player/Blueprint/FirstPersonCharacter.QTE` true _asfirst_person_character)
      (`SceneComponent.SetVisibility` (`/Game/_UnderGround/Player/Blueprint/FirstPersonCharacter.torch` _asfirst_person_character) false false)
      (`|ExecutionSequence`
        (:`then_0`
          (bind _outactor (`LevelSequencePlayer.CreateLevelSequencePlayer` (`self.MySequence`)))
          (`MovieSceneSequencePlayer.Play` (`LevelSequenceActor.SequencePlayer` _outactor)))
        (:`then_1`
          (`PrimitiveComponent.SetCollisionResponseToAllChannels` (`self.Box1`) "ECR_Block")
          (bind _asfirst_person_character_2 (cast `/Game/_UnderGround/Player/Blueprint/FirstPersonCharacter` (`GameplayStatics.GetPlayerCharacter` 0)))
          (bind (_returnvalue_x _returnvalue_y _returnvalue_z) (`KismetMathLibrary.BreakVector` (`SceneComponent.K2_GetComponentLocation` (`Character.CapsuleComponent` _asfirst_person_character_2))))
          (`SceneComponent.K2_SetWorldLocation` (`Character.CapsuleComponent` _asfirst_person_character_2) (`KismetMathLibrary.MakeVector` (- _returnvalue_x 900.0) _returnvalue_y _returnvalue_z) false false))
        (:`then_2`
          (`KismetSystemLibrary.Delay` 11.0)
          (bind _asfirst_person_character_3 (cast `/Game/_UnderGround/Player/Blueprint/FirstPersonCharacter` (`GameplayStatics.GetPlayerPawn` 0)))
          (set `/Game/_UnderGround/Player/Blueprint/FirstPersonCharacter.QTE` false _asfirst_person_character_3)
          (`SceneComponent.SetVisibility` (`/Game/_UnderGround/Player/Blueprint/FirstPersonCharacter.torch` _asfirst_person_character_3) true false))))))

(fn `UserConstructionScript`)