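; BP_TriggerDoorEvent is a one-shot trigger that plays a door-closing cinematic and shuts the level's gates.
; When the FirstPersonCharacter's capsule (matched by display name) enters the Box, it plays ClooseSequence and sets the character's QTE flag, cleared after a fixed delay.
; Meanwhile it calls CloseTrigger on every BP_Gate and sets BoxTrigger inside that loop to block retriggering.
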(event `self.Box.OnComponentBeginOverlap`
  (params (OverlappedComponent :type "PrimitiveComponent Object Reference") (OtherActor :type "Actor Object Reference") (OtherComp :type "PrimitiveComponent Object Reference") (OtherBodyIndex :type Integer) (bFromSweep :type Boolean) (SweepResult :type "HitResult Structure (by ref)"))
  (if (not (`self.BoxTrigger`))
    (bind _asfirst_person_character (cast `/Game/_UnderGround/Player/Blueprint/FirstPersonCharacter` OtherActor))
    (if (`KismetStringLibrary.EqualEqual_StrStr` (`KismetSystemLibrary.GetDisplayName` (`Character.CapsuleComponent` _asfirst_person_character)) (`KismetSystemLibrary.GetDisplayName` OtherComp))
      (`KismetSystemLibrary.PrintString` "FermeToi")
      (bind _outactor (`LevelSequencePlayer.CreateLevelSequencePlayer` (`self.ClooseSequence`)))
      (set `/Game/_UnderGround/Player/Blueprint/FirstPersonCharacter.QTE` true _asfirst_person_character)
      (`MovieSceneSequencePlayer.Play` (`LevelSequenceActor.SequencePlayer` _outactor))
      (`|ExecutionSequence`
        (:`then_0`
          (`KismetSystemLibrary.Delay` 11.5)
          (set `/Game/_UnderGround/Player/Blueprint/FirstPersonCharacter.QTE` false _asfirst_person_character))
        (:`then_1`
          (bind _outactors (`GameplayStatics.GetAllActorsOfClass` "/Game/_UnderGround/Mechanics/BP_Gate.BP_Gate_C"))
          (for _array_element _outactors
            (`/Game/_UnderGround/Mechanics/BP_Gate.CloseTrigger` _array_element)
            (set `self.BoxTrigger` true)))))))

(fn `UserConstructionScript`)