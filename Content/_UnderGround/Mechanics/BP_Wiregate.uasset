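; BP_Wiregate is a gate Blueprint, apparently meant to move vertically when a wire is placed, though its WirePlaced event is empty.
; BeginPlay caches the gate's relative location and default height.
; An unconnected Timeline chain sets Height to HeightMax and lerps the Z offset from the default, moving Box and Gate together.
; Nothing triggers that chain, so the gate stays still as written.
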(event `WirePlaced`)

(event `self.ReceiveBeginPlay`
  (bind _returnvalue_location (`KismetMathLibrary.BreakTransform` (`SceneComponent.GetRelativeTransform` (`self.gate`))))
  (set `self.DoorPos` _returnvalue_location)
  (set `self.DefaultHeight` (`self.Height`)))

(fn `UserConstructionScript`
  (`parent.UserConstructionScript`))