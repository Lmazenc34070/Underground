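; BP_Gate is a sliding gate that raises and lowers through timeline-driven Lerps of its height, with sound.
; OpeningTrigger raises it fully when powered (Alimented), or plays a partial opening until a first-try flag is set.
; CloseTrigger lowers it once and blocks later openings; both triggers are ignored for wire doors.
; WirePlaced runs a separate timeline that nudges the Box component upward each update rather than interpolating the gate.
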(event `CloseTrigger`
  (bind (_doorpos_x _doorpos_y _doorpos_z) (`KismetMathLibrary.BreakVector` (`self.DoorPos`)))
  (bind _returnvalue_location (`KismetMathLibrary.BreakTransform` (`SceneComponent.GetRelativeTransform` (`self.gate`))))
  (if (not (`self.WireDoor`))
    (if (not (`self.DoorClose`))
      (set `self.StartClose` true)
      (bind _output_get (set `self.Height` (`self.HeightMax2`)))
      (`GameplayStatics.PlaySoundAtLocation` "/Game/_UnderGround/Sounds/Gate.Gate" _returnvalue_location (struct) 1.0 1.0 0.0 null null null null)
      (bind (_direction _movement) (`Timeline|Timeline_2`)
        (:`Update`
          (`SceneComponent.K2_SetRelativeLocation` (`self.gate`) (`KismetMathLibrary.MakeVector` _doorpos_x _doorpos_y (- _doorpos_z (`KismetMathLibrary.Lerp` (`self.DefaultHeight`) _output_get _movement))) false false)
          (set `self.DoorClose` true))))))

(event `OpeningTrigger`
  (params (Alimented :type Boolean))
  (bind (_doorpos_x _doorpos_y _doorpos_z) (`KismetMathLibrary.BreakVector` (`self.DoorPos`)))
  (bind _gate (`self.gate`))
  (if (`self.StartClose`)
    _
    (elif (not (`self.WireDoor`))
      (if Alimented
        (bind _output_get (set `self.Height` (`self.HeightMax`)))
        (`GameplayStatics.PlaySoundAtLocation` "/Game/_UnderGround/Sounds/Gate.Gate" (stale `self.ReceiveBeginPlay` _output_get) (struct) 1.0 1.0 0.0 null null null null)
        (bind (_direction _movement) (`Timeline|Timeline_0`)
          (:`Update`
            (`SceneComponent.K2_SetRelativeLocation` _gate (`KismetMathLibrary.MakeVector` _doorpos_x _doorpos_y (+ (`KismetMathLibrary.Lerp` (`self.DefaultHeight`) _output_get _movement) _doorpos_z)) false false)))
        (elif (not (`self.FirstStartTry`))
          (`GameplayStatics.PlaySoundAtLocation` "/Game/_UnderGround/Sounds/gat0_5.gat0_5" (stale `self.ReceiveBeginPlay` _output_get) (struct) 1.0 1.0 0.0 null null null null)
          (bind (_direction_2 _movement_2) (`Timeline|Opening`)
            (:`Update`
              (`SceneComponent.K2_SetRelativeLocation` _gate (`KismetMathLibrary.MakeVector` _doorpos_x _doorpos_y (+ (`KismetMathLibrary.Lerp` 0.0 (`self.Height`) _movement_2) _doorpos_z)) false false)
              (set `self.FirstStartTry` true))))))))

(event `self.ReceiveBeginPlay`
  (bind _returnvalue_location (`KismetMathLibrary.BreakTransform` (`SceneComponent.GetRelativeTransform` (`self.gate`))))
  (bind _output_get (set `self.DoorPos` _returnvalue_location))
  (set `self.DefaultHeight` (`self.Height`)))

(event `WirePlaced`
  (bind _returnvalue_location (`KismetMathLibrary.BreakTransform` (`SceneComponent.GetRelativeTransform` (`self.gate`))))
  (bind (_returnvalue_x _returnvalue_y _returnvalue_z) (`KismetMathLibrary.BreakVector` (`SceneComponent.K2_GetComponentLocation` (`self.Box`))))
  (`KismetSystemLibrary.PrintString` (`KismetStringLibrary.Conv_VectorToString` _returnvalue_location))
  (bind _output_get (set `self.Height` (`self.HeightMax`)))
  (bind (_direction _movement) (`Timeline|Timeline_1`)
    (:`Update`
      (`SceneComponent.K2_SetWorldLocation` (`self.Box`) (`KismetMathLibrary.MakeVector` _returnvalue_x _returnvalue_y (+ 0.1 _returnvalue_z)) false false))))

(fn `UserConstructionScript`)