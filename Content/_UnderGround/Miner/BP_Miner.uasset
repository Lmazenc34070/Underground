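; BP_Miner is an AI-controlled miner that walks to a preset location when triggered.
; LetsGOOOO waits a short random delay, sets its go flag and passes it with the target Loc to the IAC_Miner controller.
; Tick clears the flag near the target and, for the Newt variant, snaps the actor to a fixed yaw.
; The construction script also uses Newt to pick the body material.
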(event `self.ReceiveTick`
  (params (DeltaSeconds :type "Float (single-precision)"))
  (if (== (`self.Loc`) (`self.K2_GetActorLocation`) :`ErrorTolerance` 60.0)
    (set `self.OkkkkLetsGo` false)
    (if (`self.Newt`)
      (`self.K2_SetActorRelativeRotation` (struct :`Yaw` 110.0)))))

(event `LetsGOOOO`
  (`KismetSystemLibrary.Delay` (`KismetMathLibrary.RandomFloatInRange` 0.0 0.3))
  (set `self.OkkkkLetsGo` true)
  (bind _asiac_miner (cast `/Game/_UnderGround/Miner/IAC_Miner` (`self.GetController`)))
  (`/Game/_UnderGround/Miner/IAC_Miner.LetsGoTousEnzemble` _asiac_miner (`self.OkkkkLetsGo`) (`self.Loc`)))

(fn `UserConstructionScript`
  (bind _mesh (`self.Mesh`))
  (if (`self.Newt`)
    (`PrimitiveComponent.SetMaterial` _mesh 1 "/Game/_UnderGround/Newt/Modd/Body_N.Body_N")
    (else
      (`PrimitiveComponent.SetMaterial` _mesh 1 "/Game/_UnderGround/Newt/Modd/Ch17_body.Ch17_body"))))