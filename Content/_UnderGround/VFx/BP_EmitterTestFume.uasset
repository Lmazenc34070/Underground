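; Test smoke emitter trap that sprays a Niagara smoke effect when the first-person character walks into it.
; Box overlap by the character's capsule calls Enfumage, which activates the smoke and plays a one-second hiss sound.
; The capsule leaving the Sphere deactivates the smoke and clears the Activate flag that blocks retriggering.
; Debug prints remain, and a random-chance roll is left unwired.
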(event `Enfumage`
  (`KismetSystemLibrary.PrintString` "Dans le pif")
  (`ActorComponent.Activate` (`self.NS_Test_FumeEmiter_System`) false)
  (`AudioComponent.Play` (`self.PS4_pchit_fumee`) 0.0)
  (`KismetSystemLibrary.Delay` 1.0)
  (`AudioComponent.Stop` (`self.PS4_pchit_fumee`)))

(event `self.Box.OnComponentBeginOverlap`
  (params (OverlappedComponent :type "PrimitiveComponent Object Reference") (OtherActor :type "Actor Object Reference") (OtherComp :type "PrimitiveComponent Object Reference") (OtherBodyIndex :type Integer) (bFromSweep :type Boolean) (SweepResult :type "HitResult Structure (by ref)"))
  (if (not (`self.Activate`))
    (bind _asfirst_person_character (cast `/Game/_UnderGround/Player/Blueprint/FirstPersonCharacter` OtherActor))
    (if (`KismetStringLibrary.EqualEqual_StrStr` (`KismetSystemLibrary.GetDisplayName` (`Character.CapsuleComponent` _asfirst_person_character)) (`KismetSystemLibrary.GetDisplayName` OtherComp))
      (`KismetSystemLibrary.PrintString` "Dans le pif")
      (`self.Enfumage`)
      (set `self.Activate` true))))

(event `self.Sphere.OnComponentEndOverlap`
  (params (OverlappedComponent :type "PrimitiveComponent Object Reference") (OtherActor :type "Actor Object Reference") (OtherComp :type "PrimitiveComponent Object Reference") (OtherBodyIndex :type Integer))
  (bind _asfirst_person_character (cast `/Game/_UnderGround/Player/Blueprint/FirstPersonCharacter` OtherActor))
  (if (`KismetStringLibrary.EqualEqual_StrStr` (`KismetSystemLibrary.GetDisplayName` (`Character.CapsuleComponent` _asfirst_person_character)) (`KismetSystemLibrary.GetDisplayName` OtherComp))
    (`ActorComponent.Deactivate` (`self.NS_Test_FumeEmiter_System`))
    (set `self.Activate` false)))

(fn `UserConstructionScript`)