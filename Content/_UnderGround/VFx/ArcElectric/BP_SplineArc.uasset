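; BP_SplineArc is an electric arc VFX actor that stretches a two-point spline between the player's SphereStart component and the character's EndVfx location.
; Each Tick it casts to FirstPersonCharacter and moves both spline endpoints to those world positions.
; It wobbles the arc by easing each point's local Y tangent toward a random target, with opposing vertical tangents.
; It also prints the horizontal endpoint distance every frame as debug output.
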(event `self.ReceiveBeginPlay`)

(event `self.ReceiveTick`
  (params (DeltaSeconds :type "Float (single-precision)"))
  (bind _spline (`self.Spline`))
  (bind _spline_2 (`self.Spline`))
  (bind _spline_3 (`self.Spline`))
  (bind (_returnvalue_x _returnvalue_y) (`KismetMathLibrary.BreakVector` (`SplineComponent.GetTangentAtSplinePoint` _spline 1 "Local")))
  (bind (_returnvalue_x_2 _returnvalue_y_2) (`KismetMathLibrary.BreakVector` (`SplineComponent.GetTangentAtSplinePoint` _spline_3 0 "Local")))
  (bind _asfirst_person_character (cast `/Game/_UnderGround/Player/Blueprint/FirstPersonCharacter` (`GameplayStatics.GetPlayerCharacter` 0)))
  (`SplineComponent.SetLocationAtSplinePoint` _spline_2 0 (`SceneComponent.K2_GetComponentLocation` (`/Game/_UnderGround/Player/Blueprint/FirstPersonCharacter.SphereStart` _asfirst_person_character)) "World" true)
  (`SplineComponent.SetLocationAtSplinePoint` _spline_2 1 (`/Game/_UnderGround/Player/Blueprint/FirstPersonCharacter.EndVfx` _asfirst_person_character) "World" true)
  (`SplineComponent.SetTangentAtSplinePoint` _spline_3 0 (`KismetMathLibrary.MakeVector` 0.0 (`KismetMathLibrary.FInterpTo` _returnvalue_y_2 (`KismetMathLibrary.RandomFloatInRange` -250.0 250.0) (`GameplayStatics.GetWorldDeltaSeconds`) 1.0) 250.0) "Local" true)
  (`SplineComponent.SetTangentAtSplinePoint` _spline_3 1 (`KismetMathLibrary.MakeVector` 0.0 (`KismetMathLibrary.FInterpTo` _returnvalue_y (`KismetMathLibrary.RandomFloatInRange` -250.0 250.0) (`GameplayStatics.GetWorldDeltaSeconds`) 1.0) -250.0) "Local" true)
  (`KismetSystemLibrary.PrintString` (`KismetStringLibrary.Conv_DoubleToString` (`KismetMathLibrary.VSizeXY` (- (`SplineComponent.GetLocationAtSplinePoint` _spline 0 "World") (`SplineComponent.GetLocationAtSplinePoint` _spline 1 "World")))) true true (struct :`G` 0.66 :`B` 1.0 :`A` 1.0) 0.0))

(fn `UserConstructionScript`)