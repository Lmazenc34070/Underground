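; Electric arc effect actor that renders a beam particle with moving endpoints.
; On BeginPlay, the Movement timeline incrementally offsets the Start component along local X and the End component along local Y.
; Every tick, End's world location is written to the ElectricArcs particle's BeamEnd vector parameter so the beam tracks it.
; An unconnected cast to FirstPersonCharacter never runs.
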(event `self.ReceiveBeginPlay`
  (bind (_direction _movement) (`Timeline|Movement`)
    (:`Update`
      (`SceneComponent.K2_AddLocalOffset` (`self.Start`) (`KismetMathLibrary.MakeVector` _movement) false true)
      (`SceneComponent.K2_AddLocalOffset` (`self.End`) (`KismetMathLibrary.MakeVector` 0.0 _movement) false true))))

(event `self.ReceiveTick`
  (params (DeltaSeconds :type "Float (single-precision)"))
  (`FXSystemComponent.SetVectorParameter` (`self.ElectricArcs`) "BeamEnd" (`SceneComponent.K2_GetComponentLocation` (`self.End`))))

(fn `UserConstructionScript`)